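; Ammo pickup actor that refills a matching weapon carried by the character who collects it.
; On BeginPlay it binds to its Pickup component's OnPickUp event.
; The handler searches the character's attached actors recursively for a TP_WeaponComponent with the same AmmoType, adds AmmoAmount to its Ammo and destroys the pickup.
; Debug strings print each attached actor's name and any missing-weapon or wrong-type case.
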(event `self.ReceiveBeginPlay`
  (add `TP_PickUpComponent.OnPickUp` (`self.Pickup`) (delegate `OnPickup`)))

(event `OnPickup`
  (params (PickUpCharacter :type "SpaceEggCharacter Object Reference"))
  (for _array_element (`self.GetAttachedActors` PickUpCharacter true true)
    (`KismetSystemLibrary.PrintString` (`KismetSystemLibrary.GetDisplayName` _array_element))
    (bind _returnvalue (`self.GetComponentByClass` _array_element "/Script/SpaceEgg.TP_WeaponComponent"))
    (`/Engine/EditorBlueprintResources/StandardMacros.IsValid` _returnvalue
      (:`Is Valid`
        (if (`KismetStringLibrary.EqualEqual_StrStr` (`TP_WeaponComponent.AmmoType` _returnvalue) (`self.AmmoType`))
          (set `TP_WeaponComponent.Ammo` (+ (`TP_WeaponComponent.Ammo` _returnvalue) (`self.AmmoAmount`)) _returnvalue)
          (`self.K2_DestroyActor`)
          (else
            (`KismetSystemLibrary.PrintString` "Wrong Ammo Type"))))
      (:`Is Not Valid`
        (`KismetSystemLibrary.PrintString` "No Weapon")))))

(fn `UserConstructionScript`)