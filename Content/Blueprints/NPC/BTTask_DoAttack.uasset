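; Behavior tree task that makes an NPC perform a named attack against an actor taken from the blackboard.
; On its Tick event, it casts the owner to SpaceEggNPCAIController and calls DoAttack on that NPC's Attack member with AttackName and the ActorToAttack value.
; The task finishes with the attack's result, or fails if the owner is invalid or not that controller type.
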(event `self.ReceiveTick`
  (params (OwnerActor :type "Actor Object Reference") (DeltaSeconds :type "Float (single-precision)"))
  (`/Engine/EditorBlueprintResources/StandardMacros.IsValid` OwnerActor
    (:`Is Valid`
      (bind _asspace_egg_npcaicontroller (cast `SpaceEggNPCAIController` OwnerActor)
        (:`then`
          (bind _returnvalue (`NPCAttackComponent.DoAttack` (`SpaceEggNPC.Attack` (`SpaceEggNPCAIController.GetNPC` _asspace_egg_npcaicontroller)) (`self.AttackName`) (`BTFunctionLibrary.GetBlackboardValueAsActor` (`self.ActorToAttack`))))
          (`self.FinishExecute` _returnvalue))
        (:`CastFailed`
          (`self.FinishExecute` false))))
    (:`Is Not Valid`
      (`self.FinishExecute` false))))